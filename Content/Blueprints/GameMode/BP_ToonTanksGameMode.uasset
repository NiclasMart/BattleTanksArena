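; Game mode Blueprint for Toon Tanks that shows the start and end screens of each round.
; StartGame creates the start widget, passes it the start delay as its countdown and labels it with the current and total round numbers.
; EndGame shows the end widget with a game over, round won or all-rounds-finished message, based on the GameOver flag and round count.
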(event `self.StartGame`
  (bind _returnvalue (`|CreateWidget` "/Game/Blueprints/Widgets/WBP_GameStartWidget.WBP_GameStartWidget_C"))
  (set `/Game/Blueprints/Widgets/WBP_GameStartWidget.Countdown` (`self.GameStartDelayTime`) _returnvalue)
  (`TextBlock.SetText` (`/Game/Blueprints/Widgets/WBP_GameStartWidget.RoundDisplay` _returnvalue) (`KismetTextLibrary.Conv_StringToText` (`KismetStringLibrary.Concat_StrStr` "ROUND " (`KismetStringLibrary.Conv_IntToString` (`self.CurrentRound`)) "-" (`KismetStringLibrary.Conv_IntToString` (`self.TotalRoundCount`)))))
  (`UserWidget.AddToViewport` _returnvalue 0))

(event `self.EndGame`
  (params (bGameOver :type Boolean))
  (bind _returnvalue (`|CreateWidget` "/Game/Blueprints/Widgets/WBP_GameEndWidget.WBP_GameEndWidget_C"))
  (`UserWidget.AddToViewport` _returnvalue 0)
  (`TextBlock.SetText` (`/Game/Blueprints/Widgets/WBP_GameEndWidget.DisplayText` _returnvalue) (`KismetTextLibrary.Conv_StringToText` (select `bool` (and (== (`self.CurrentRound`) (`self.TotalRoundCount`)) (not bGameOver)) :`false` (select `bool` bGameOver :`false` "You Have Won!" :`true` "Game Over!") :`true` "Finished All Rounds! Congratulation"))))

(fn `UserConstructionScript`)